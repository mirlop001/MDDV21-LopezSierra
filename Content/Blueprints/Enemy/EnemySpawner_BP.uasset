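; Enemy spawner actor that creates a per-level quota of enemies at its own location.
; Each Tick it compares its spawn counter with the FirstPersonGameMode's EnemiesPerLevel times CurrentLevel, incrementing it and attempting a spawn while below that.
; SpawnPickup spawns a random ItemtoSpawn class, adjusting for collisions but always spawning.
; It then clears CurrentItem instead of storing the new actor, so the validity guard does not track spawns.
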(event `self.ReceiveTick`
  (params (DeltaSeconds :type "Float (single-precision)"))
  (bind _asfirst_person_game_mode (cast `/Game/FirstPersonBP/Blueprints/FirstPersonGameMode` (`GameplayStatics.GetGameMode`)))
  (if (< (`self.NumEnemiesSpawned`) (* (`/Game/FirstPersonBP/Blueprints/FirstPersonGameMode.EnemiesPerLevel` _asfirst_person_game_mode) (`/Game/FirstPersonBP/Blueprints/FirstPersonGameMode.CurrentLevel` _asfirst_person_game_mode)))
    (`/Engine/EditorBlueprintResources/StandardMacros.IncrementInt` (`self.NumEnemiesSpawned`)
      (:`  `
        (`self.AttemptToSpawn`)))))

(fn `AttemptToSpawn`
  (`/Engine/EditorBlueprintResources/StandardMacros.IsValid` (`self.CurrentItem`)
    (:`Is Not Valid`
      (`self.SpawnPickup`))))

(fn `SpawnPickup`
  (`|SpawnActorFromClass` (`|GetArrayItem` (`self.ItemtoSpawn`) (`KismetMathLibrary.RandomIntegerInRange` 0 (- (`KismetArrayLibrary.Array_Length` (`self.ItemtoSpawn`)) 1))) (`KismetMathLibrary.MakeTransform` (`self.K2_GetActorLocation`) (`self.K2_GetActorRotation`)) "AdjustIfPossibleButAlwaysSpawn" "OverrideRootScale" self null)
  (set `self.CurrentItem` null))

(fn `UserConstructionScript`)