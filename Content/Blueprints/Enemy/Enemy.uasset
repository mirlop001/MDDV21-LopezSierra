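; Ghost enemy Blueprint that patrols, turns angry when shot, and dies on the second projectile hit.
; Tick moves it back and forth, flipping Direccion through a three-second Delay, until Tocado is set, then interpolates it toward the player and copies the player's rotation.
; Hit handles projectiles by spawning effects, changing the ghost's face or destroying it and incrementing the player's EnemiesDefeated.
; Hitting the player character instead reduces its Health and shows the eyebrows and SKFPGun.
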(event `self.ReceiveHit`
  (params (MyComp :type "PrimitiveComponent Object Reference") (Other :type "Actor Object Reference") (OtherComp :type "PrimitiveComponent Object Reference") (bSelfMoved :type Boolean) (HitLocation :type "Vector Structure") (HitNormal :type "Vector Structure") (NormalImpulse :type "Vector Structure") (Hit :type "HitResult Structure (by ref)"))
  (bind _asfirst_person_projectile (cast `/Game/FirstPersonBP/Blueprints/FirstPersonProjectile` Other)
    (:`then`
      (`self.K2_DestroyActor` _asfirst_person_projectile)
      (`GameplayStatics.SpawnEmitterAtLocation` (select `bool` (`self.Tocado`) :`true` "/Game/StarterContent/Particles/P_Explosion.P_Explosion" :!type "ParticleSystem Object Reference") HitLocation)
      (if (`self.Tocado`)
        (`self.K2_DestroyActor`)
        (bind _asfirst_person_character (cast `/Game/FirstPersonBP/Blueprints/FirstPersonCharacter` (`GameplayStatics.GetPlayerPawn` 0)))
        (`/Engine/EditorBlueprintResources/StandardMacros.IncrementInt` (`/Game/FirstPersonBP/Blueprints/FirstPersonCharacter.EnemiesDefeated` _asfirst_person_character))
        (else
          ;[1 1 1] Comment
          (`SceneComponent.SetVisibility` (`self.Eyebrow`) true false)
          (`SceneComponent.SetVisibility` (`self.Eyebrow2`) true false)
          (`PrimitiveComponent.SetMaterial` (`self.Body`) 0 "/Engine/Angry_ghost_material.Angry_ghost_material")
          (set `self.Tocado` true))))
    (:`CastFailed`
      ;[1 1 1] Enemy hits FPC
      (bind _asfirst_person_character_2 (cast `/Game/FirstPersonBP/Blueprints/FirstPersonCharacter` Other))
      (`SceneComponent.SetVisibility` (`self.Eyebrow`) true false)
      (`SceneComponent.SetVisibility` (`self.Eyebrow2`) true false)
      (`SceneComponent.SetVisibility` (`self.SK_FPGun`) true false)
      (set `/Game/FirstPersonBP/Blueprints/FirstPersonCharacter.Health` (- (`/Game/FirstPersonBP/Blueprints/FirstPersonCharacter.Health` _asfirst_person_character_2) 5.0) _asfirst_person_character_2))))

(event `self.ReceiveTick`
  (params (DeltaSeconds :type "Float (single-precision)"))
  (bind _returnvalue (`GameplayStatics.GetPlayerPawn` 0))
  ;[1 1 1] Enemy movement and direction settings
  (if (`self.Tocado`)
    ;;[1 1 1] Ghost follows the main character
    (`self.K2_SetActorLocation` (`KismetMathLibrary.VInterpTo` (`self.K2_GetActorLocation`) (`self.K2_GetActorLocation` _returnvalue) DeltaSeconds 2.0))
    (`self.K2_SetActorRotation` (`self.K2_GetActorRotation` _returnvalue))
    (else
      ;;[1 1 1] Ghost moves on its way
      (`self.K2_AddActorWorldOffset` (* (`KismetMathLibrary.Normal` (`self.Direccion`)) (* DeltaSeconds (`self.Velocidad`))))
      ;;[1 1 1] Direction changes every 3 sec
      (`KismetSystemLibrary.Delay` 3.0)
      (set `self.Direccion` (* (`self.Direccion`) -1.0)))))

(fn `UserConstructionScript`)